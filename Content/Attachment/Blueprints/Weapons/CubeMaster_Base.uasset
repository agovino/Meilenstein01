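; CubeMaster_Base is a hand-held modular weapon base that carries attachments in child-actor AttachmentSlots.
; Pickup snaps the mesh to the hand and, if the other hand holds an attachment, spawns ghost copies of it at free slots of the matching type.
; Drop by the holding hand restores physics, detaches and destroys the ghosts.
; Trigger, face button, grip and thumbstick presses and releases are forwarded to every attachment in a used slot.
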(event `/Game/Attachment/Blueprints/Pickup.Pickup`
  (params (Hand :type "/Game/Attachment/Blueprints/BP_MotionController Object Reference"))
  (bind _staticmesh (`self.StaticMesh`))
  ;[1 1 1] Base Pickup
  (`|ExecutionSequence`
    (:`then_0`
      (bind _asattachment_base (cast `/Game/Attachment/Blueprints/Attachments/Attachment_Base` (`/Game/Attachment/Blueprints/BP_MotionController.GrabObject` (`/Game/Attachment/Blueprints/BP_MotionController.OtherHand` Hand))))
      (`self.ShowSlots` (`/Game/Attachment/Blueprints/Attachments/Attachment_Base.Slot` _asattachment_base) (`GameplayStatics.GetObjectClass` _asattachment_base)))
    (:`then_1`
      (`PrimitiveComponent.SetSimulatePhysics` _staticmesh false)
      (`SceneComponent.K2_AttachToComponent` _staticmesh (`/Game/Attachment/Blueprints/BP_MotionController.HandMesh` Hand) (`self.Socket`) "SnapToTarget" "SnapToTarget" "KeepWorld" true))))

(event `/Game/Attachment/Blueprints/Pickup.Drop`
  (params (Hand :type "/Game/Attachment/Blueprints/BP_MotionController Object Reference"))
  (bind _staticmesh (`self.StaticMesh`))
  ;[1 1 1] Base Drop
  (if (== (`self.GetAttachActor`) Hand)
    (`PrimitiveComponent.SetSimulatePhysics` _staticmesh true)
    (`SceneComponent.K2_DetachFromComponent` _staticmesh "KeepWorld" "KeepWorld" "KeepWorld" true)
    (`self.HideSlots`)))

(event `/Game/Attachment/Blueprints/Input.TriggerPress`
  ;[1 1 1] Trigger
  (for _array_element (`self.GetAttachments`)
    (`/Game/Attachment/Blueprints/Attachments/Attachment_Base.TriggerPress` _array_element)))

(event `/Game/Attachment/Blueprints/Input.TriggerRelease`
  ;[1 1 1] Trigger
  (for _array_element (`self.GetAttachments`)
    (`/Game/Attachment/Blueprints/Attachments/Attachment_Base.TriggerRelease` _array_element)))

(event `/Game/Attachment/Blueprints/Input.FaceButton1Press`
  ;[1 1 1] FaceButton1
  (for _array_element (`self.GetAttachments`)
    (`/Game/Attachment/Blueprints/Attachments/Attachment_Base.FaceButton1Press` _array_element)))

(event `/Game/Attachment/Blueprints/Input.FaceButton1Release`
  ;[1 1 1] FaceButton1
  (for _array_element (`self.GetAttachments`)
    (`/Game/Attachment/Blueprints/Attachments/Attachment_Base.FaceButton1Release` _array_element)))

(event `/Game/Attachment/Blueprints/Input.FaceButton2Press`
  ;[1 1 1] FaceButton2
  (for _array_element (`self.GetAttachments`)
    (`/Game/Attachment/Blueprints/Attachments/Attachment_Base.FaceButton2Press` _array_element)))

(event `/Game/Attachment/Blueprints/Input.FaceButton2Release`
  ;[1 1 1] FaceButton2
  (for _array_element (`self.GetAttachments`)
    (`/Game/Attachment/Blueprints/Attachments/Attachment_Base.FaceButton2Release` _array_element)))

(event `/Game/Attachment/Blueprints/Input.GripPress`
  ;[1 1 1] Grip
  (for _array_element (`self.GetAttachments`)
    (`/Game/Attachment/Blueprints/Attachments/Attachment_Base.GripPress` _array_element)))

(event `/Game/Attachment/Blueprints/Input.GripRelease`
  ;[1 1 1] Grip
  (for _array_element (`self.GetAttachments`)
    (`/Game/Attachment/Blueprints/Attachments/Attachment_Base.GripRelease` _array_element)))

(event `/Game/Attachment/Blueprints/Input.ThumbstickPress`
  ;[1 1 1] Thumbstick
  (for _array_element (`self.GetAttachments`)
    (`/Game/Attachment/Blueprints/Attachments/Attachment_Base.ThumbstickPress` _array_element)))

(event `/Game/Attachment/Blueprints/Input.ThumbstickRelease`
  ;[1 1 1] Thumbstick
  (for _array_element (`self.GetAttachments`)
    (`/Game/Attachment/Blueprints/Attachments/Attachment_Base.ThumbstickRelease` _array_element)))

(fn `GetAttachActor`
  (returns (ReturnValue :type "Actor Object Reference"))
  (bind _returnvalue (`SceneComponent.GetAttachParent` (`self.StaticMesh`)))
  (bind _returnvalue_2 (`ActorComponent.GetOwner` _returnvalue))
  (`/Engine/EditorBlueprintResources/StandardMacros.IsValid` _returnvalue
    (:`Is Valid`
      (`/Engine/EditorBlueprintResources/StandardMacros.IsValid` _returnvalue_2
        (:`Is Valid`
          (return _returnvalue_2))
        (:`Is Not Valid`
          _)))
    (:`Is Not Valid`
      _))
  (return null))

(fn `GetAttachments`
  (returns (Attachments :type "Array of /Game/Attachment/Blueprints/Attachments/Attachment_Base Object Reference"))
  (locals (Temp :type "Array of /Game/Attachment/Blueprints/Attachments/Attachment_Base Object Reference"))
  (for _array_element (`self.K2_GetComponentsByClass` "/Script/Engine.ChildActorComponent")
    (bind _asattachment_slot (cast `/Game/Attachment/Blueprints/Attachments/AttachmentSlot` (`ChildActorComponent.ChildActor` _array_element)))
    (if (`/Game/Attachment/Blueprints/Attachments/AttachmentSlot.Used` _asattachment_slot)
      (`KismetArrayLibrary.Array_Add` (`local.Temp`) (`/Game/Attachment/Blueprints/Attachments/AttachmentSlot.Attachment` _asattachment_slot))))
  (return (`local.Temp`)))

(fn `HideSlots`
  (for _array_element (`self.Ghosts`)
    (`/Engine/EditorBlueprintResources/StandardMacros.IsValid` _array_element
      (:`Is Valid`
        (`self.K2_DestroyActor` _array_element)))))

(fn `ShowSlots`
  (params (Slot :type Name) (Ghost :type "/Game/Attachment/Blueprints/Attachments/Attachment_Base Class Reference"))
  (for _array_element (`self.K2_GetComponentsByClass` "/Script/Engine.ChildActorComponent")
    (bind _asattachment_slot (cast `/Game/Attachment/Blueprints/Attachments/AttachmentSlot` (`ChildActorComponent.ChildActor` _array_element)))
    (if (and (== (`/Game/Attachment/Blueprints/Attachments/AttachmentSlot.Slot` _asattachment_slot) Slot) (not (`/Game/Attachment/Blueprints/Attachments/AttachmentSlot.Used` _asattachment_slot)))
      (bind _returnvalue (`|SpawnActorFromClass` Ghost (`SceneComponent.K2_GetComponentToWorld` _array_element) "Undefined" "OverrideRootScale" null true null))
      (`self.K2_AttachToComponent` _returnvalue _array_element "None" "SnapToTarget" "SnapToTarget" "KeepWorld" true)
      (`KismetArrayLibrary.Array_Add` (`self.Ghosts`) _returnvalue))))

(fn `UserConstructionScript`)