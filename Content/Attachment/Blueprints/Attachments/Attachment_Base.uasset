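; Base actor for weapon attachments that are picked up by hand and mounted on weapon attachment slots.
; Pickup frees it from any slot, snaps its mesh to the hand and shows matching slots on a weapon in the other hand, passing its own class for ghost previews.
; Drop restores physics if the hand still holds it and hides those slots.
; With the Ghost flag set, construction swaps all static mesh materials to a ghost material and disables physics.
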(event `Attached`
  (params (Weapon :type "/Game/Attachment/Blueprints/Weapons/Weapon_Base Object Reference"))
  ;[1 1 1] Base Attach Event
  (set `self.Weapon` Weapon) ; Object Type
  (`PrimitiveComponent.SetCollisionEnabled` (`self.StaticMesh`) "QueryOnly")
  (`PrimitiveComponent.SetSimulatePhysics` (`self.StaticMesh`) false))

(event `Detached`
  (params (Weapon :type "/Game/Attachment/Blueprints/Weapons/Weapon_Base Object Reference"))
  ;[1 1 1] Base Attach Event
  (set `self.Weapon` null) ; Object Type
  (`PrimitiveComponent.SetCollisionEnabled` (`self.StaticMesh`) "QueryAndPhysics"))

(event `/Game/Attachment/Blueprints/Pickup.Pickup`
  (params (Hand :type "/Game/Attachment/Blueprints/BP_MotionController Object Reference"))
  (bind _staticmesh (`self.StaticMesh`))
  ;[1 1 1] Base Pickup
  (`|ExecutionSequence`
    (:`then_0`
      (bind _asattachment_slot (cast `/Game/Attachment/Blueprints/Attachments/AttachmentSlot` (`self.GetAttachActor`)))
      (`self.Detached` null)
      (`/Game/Attachment/Blueprints/Attachments/AttachmentSlot.Detached` _asattachment_slot))
    (:`then_1`
      (`PrimitiveComponent.SetSimulatePhysics` _staticmesh false)
      (`SceneComponent.K2_AttachToComponent` _staticmesh (`/Game/Attachment/Blueprints/BP_MotionController.HandMesh` Hand) (`self.Socket`) "SnapToTarget" "SnapToTarget" "KeepWorld" true))
    (:`then_2`
      (bind _asweapon_base (cast `/Game/Attachment/Blueprints/Weapons/Weapon_Base` (`/Game/Attachment/Blueprints/BP_MotionController.GrabObject` (`/Game/Attachment/Blueprints/BP_MotionController.OtherHand` Hand))))
      (`/Game/Attachment/Blueprints/Weapons/Weapon_Base.ShowSlots` _asweapon_base (`self.Slot`) (`GameplayStatics.GetObjectClass` self)))))

(event `/Game/Attachment/Blueprints/Pickup.Drop`
  (params (Hand :type "/Game/Attachment/Blueprints/BP_MotionController Object Reference"))
  (bind _staticmesh (`self.StaticMesh`))
  ;[1 1 1] Base Drop
  (`|ExecutionSequence`
    (:`then_0`
      (if (== (`self.GetAttachActor`) Hand)
        (`PrimitiveComponent.SetSimulatePhysics` _staticmesh true)
        (`SceneComponent.K2_DetachFromComponent` _staticmesh "KeepWorld" "KeepWorld" "KeepWorld" true)))
    (:`then_1`
      (bind _asweapon_base (cast `/Game/Attachment/Blueprints/Weapons/Weapon_Base` (`/Game/Attachment/Blueprints/BP_MotionController.GrabObject` (`/Game/Attachment/Blueprints/BP_MotionController.OtherHand` Hand))))
      (`/Game/Attachment/Blueprints/Weapons/Weapon_Base.HideSlots` _asweapon_base))))

(fn `GenerateGhost`
  (if (`self.Ghost`)
    (for _array_element (`self.K2_GetComponentsByClass` "/Script/Engine.StaticMeshComponent")
      (for _index (range (`PrimitiveComponent.GetNumMaterials` _array_element))
        (`PrimitiveComponent.SetMaterial` _array_element _index "/Game/Attachment/Materials/M_Ghost.M_Ghost")))))

(fn `GetAttachActor`
  (returns (ReturnValue :type "Actor Object Reference"))
  (bind _returnvalue (`SceneComponent.GetAttachParent` (`self.StaticMesh`)))
  (bind _returnvalue_2 (`ActorComponent.GetOwner` _returnvalue))
  (`/Engine/EditorBlueprintResources/StandardMacros.IsValid` _returnvalue
    (:`Is Valid`
      (`/Engine/EditorBlueprintResources/StandardMacros.IsValid` _returnvalue_2
        (:`Is Valid`
          (return _returnvalue_2))
        (:`Is Not Valid`
          _)))
    (:`Is Not Valid`
      _))
  (return null))

(fn `UserConstructionScript`
  (if (`self.Ghost`)
    (`self.GenerateGhost`)
    (`PrimitiveComponent.SetSimulatePhysics` (`self.StaticMesh`) false)))