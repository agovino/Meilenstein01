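; Laser sight weapon attachment that shows a beam and a dot of light where it points, toggled by face button 1.
; Each tick, unless it is a ghost, it line-traces forward from its Arrow, moving the point light and beam endpoint to the hit or trace end.
; Light intensity scales with hit distance.
; Ghost generation destroys both effects, and attaching enables query and physics collision on the mesh.
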(event `/Game/Attachment/Blueprints/Input.FaceButton1Press`
  (`SceneComponent.ToggleVisibility` (`self.ParticleSystem`) false)
  (`SceneComponent.ToggleVisibility` (`self.PointLight`) false))

(event `self.ReceiveTick`
  (params (DeltaSeconds :type "Float (single-precision)"))
  (bind _arrow (`self.Arrow`))
  (bind _returnvalue (`SceneComponent.K2_GetComponentLocation` _arrow))
  (`parent.ReceiveTick` DeltaSeconds)
  (if (not (`self.Ghost`))
    (bind _outhit (`KismetSystemLibrary.LineTraceSingle` _returnvalue (+ _returnvalue (* (`KismetMathLibrary.Conv_RotatorToVector` (`SceneComponent.K2_GetComponentRotation` _arrow)) 4000.0)) "TraceTypeQuery1"))
    (bind (_bblockinghit _binitialoverlap _time _distance _location _impactpoint _normal _impactnormal _physmat _hitactor _hitcomponent _hitbonename _hititem _faceindex _tracestart _traceend) (`GameplayStatics.BreakHitResult` _outhit))
    (bind _returnvalue_2 (`KismetMathLibrary.SelectVector` (+ _location _normal) _traceend _bblockinghit))
    (`SceneComponent.K2_SetWorldLocation` (`self.PointLight`) _returnvalue_2 false false)
    (`LightComponent.SetIntensity` (`self.PointLight`) (* _time 50.0))
    (`ParticleSystemComponent.SetBeamEndPoint` (`self.ParticleSystem`) 0 _returnvalue_2)))

(event `self.GenerateGhost`
  (`parent.GenerateGhost`)
  (`ActorComponent.K2_DestroyComponent` (`self.ParticleSystem`))
  (`ActorComponent.K2_DestroyComponent` (`self.PointLight`)))

(event `self.Attached`
  (params (Weapon :type "/Game/Attachment/Blueprints/Weapons/Weapon_Base Object Reference"))
  (`parent.Attached` Weapon)
  (`PrimitiveComponent.SetCollisionEnabled` (`self.StaticMesh`) "QueryAndPhysics"))

(fn `UserConstructionScript`
  (`parent.UserConstructionScript`))