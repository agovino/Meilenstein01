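; AttachmentSlot is an actor that snaps matching attachments onto a weapon through a sphere trigger sized by its Radius.
; On overlap, a free slot accepts a non-ghost Attachment_Base of the same slot type not already in another slot, disabling its physics and snapping its mesh to the sphere.
; It then notifies the attachment of the parent weapon and hides that weapon's slots.
; Attach and detach events play sounds and track occupancy.
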(event `Detached`
  ;[1 1 1] Play Sound at Location Detached or Attached
  (`GameplayStatics.PlaySoundAtLocation` (`self.DetachSound`) (`SceneComponent.K2_GetComponentLocation` (`self.Sphere`)) (struct) 1.0 1.0 0.0 "/Game/Attachment/Sounds/basic.basic" null null)
  (set `self.Attachment` null)
  (set `self.Used` false))

(event `Attached`
  (params (Attachment :type "/Game/Attachment/Blueprints/Attachments/Attachment_Base Object Reference"))
  ;[1 1 1] Play Sound at Location Detached or Attached
  (`GameplayStatics.PlaySoundAtLocation` (`self.AttachSound`) (`SceneComponent.K2_GetComponentLocation` (`self.Sphere`)) (struct) 1.0 1.0 0.0 "/Game/Attachment/Sounds/basic.basic" null null)
  (set `self.Attachment` Attachment)
  (set `self.Used` true))

(event `self.Sphere.OnComponentBeginOverlap`
  (params (OverlappedComponent :type "PrimitiveComponent Object Reference") (OtherActor :type "Actor Object Reference") (OtherComp :type "PrimitiveComponent Object Reference") (OtherBodyIndex :type Integer) (bFromSweep :type Boolean) (SweepResult :type "HitResult Structure (by ref)"))
  ;[1 1 1] Overlap Slot
  (bind _asattachment_base (cast `/Game/Attachment/Blueprints/Attachments/Attachment_Base` OtherActor))
  (cast `/Game/Attachment/Blueprints/Attachments/AttachmentSlot` (`self.GetAttachParentActor` _asattachment_base)
    (:`CastFailed`
      (if (and (== (`/Game/Attachment/Blueprints/Attachments/Attachment_Base.Slot` _asattachment_base) (`self.Slot`)) (not (`self.Used`)) (not (`/Game/Attachment/Blueprints/Attachments/Attachment_Base.Ghost` _asattachment_base)))
        (`self.K2_DetachFromActor` _asattachment_base "KeepWorld" "KeepWorld" "KeepWorld")
        (`self.Attached` _asattachment_base)
        (bind _staticmesh (`/Game/Attachment/Blueprints/Attachments/Attachment_Base.StaticMesh` _asattachment_base))
        (`PrimitiveComponent.SetSimulatePhysics` _staticmesh false)
        (`SceneComponent.K2_AttachToComponent` _staticmesh (`self.Sphere`) "None" "SnapToTarget" "SnapToTarget" "KeepWorld" false)
        (`|ExecutionSequence`
          (:`then_0`
            (bind _asweapon_base (cast `/Game/Attachment/Blueprints/Weapons/Weapon_Base` (`self.GetParentActor`)))
            (`/Game/Attachment/Blueprints/Attachments/Attachment_Base.Attached` (`self.Attachment`) _asweapon_base))
          (:`then_1`
            (bind _asweapon_base_2 (cast `/Game/Attachment/Blueprints/Weapons/Weapon_Base` (`self.GetAttachParentActor`)))
            (`/Game/Attachment/Blueprints/Weapons/Weapon_Base.HideSlots` _asweapon_base_2)))))))

(fn `UserConstructionScript`
  (`SphereComponent.SetSphereRadius` (`self.Sphere`) (`self.Radius`) true))