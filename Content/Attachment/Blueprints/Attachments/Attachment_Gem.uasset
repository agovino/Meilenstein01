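; Gem attachment Blueprint that extends a parent attachment class with a colored gem mesh and two point lights.
; Unless it is a ghost, the construction script creates a dynamic gem material and applies the Color variable to it and both lights.
; GenerateGhost runs the parent logic, then destroys both lights so the ghost version emits no light from them.
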(event `self.GenerateGhost`
  (`parent.GenerateGhost`)
  (`ActorComponent.K2_DestroyComponent` (`self.PointLight`))
  (`ActorComponent.K2_DestroyComponent` (`self.PointLight1`)))

(fn `UserConstructionScript`
  (bind _color (`self.Color`))
  (`parent.UserConstructionScript`)
  (if (not (`self.Ghost`))
    (bind _returnvalue (`PrimitiveComponent.CreateDynamicMaterialInstance` (`self.StaticMesh`) 0 "/Game/Attachment/Models/Gem/M_Gem.M_Gem"))
    (`MaterialInstanceDynamic.SetVectorParameterValue` _returnvalue "Color" _color)
    (`LightComponent.SetLightColor` (`self.PointLight`) _color true)
    (`LightComponent.SetLightColor` (`self.PointLight1`) _color true)))